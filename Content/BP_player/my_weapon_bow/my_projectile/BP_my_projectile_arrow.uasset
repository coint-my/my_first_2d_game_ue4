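; Arrow projectile for the player's bow that sticks into what it hits and deals point damage.
; On BeginPlay it sets the ProjectileMovement velocity to the Box's forward vector.
; When the projectile stops, it attaches to the hit actor, disables Box collision, plays an impact sound and applies damage with a custom damage type.
; It binds to the hit actor's OnDestroyed so the arrow is destroyed along with it.
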(event `self.ReceiveBeginPlay`
  (`self.set_speed_arrow` (`SceneComponent.GetForwardVector` (`self.Box`))))

(event `self.ProjectileMovement.OnProjectileStop`
  (params (ImpactResult :type "HitResult Structure (by ref)"))
  (bind (_bblockinghit _binitialoverlap _time _distance _location _impactpoint _normal _impactnormal _physmat _hitactor _hitcomponent _hitbonename _hititem _faceindex _tracestart) (`GameplayStatics.BreakHitResult` ImpactResult))
  (add `self.OnDestroyed` _hitactor (delegate `my_destroyed`))
  (`self.K2_AttachToActor` _hitactor "None" "KeepWorld" "KeepWorld" "KeepWorld")
  (`PrimitiveComponent.SetCollisionEnabled` (`self.Box`) "NoCollision")
  (`GameplayStatics.PlaySoundAtLocation` "/Game/sound/bow/s_arrow_intersect_02.s_arrow_intersect_02" (`SceneComponent.K2_GetComponentLocation` (`self.Box`)) (struct) 1.0 1.0 0.0 null null null)
  (`GameplayStatics.ApplyPointDamage` _hitactor (`self.my_damage`) _tracestart ImpactResult null null "/Game/interaction/barrel_explode/BP_my_dame_type.BP_my_dame_type_C"))

(event `my_destroyed` :!signature `self.OnDestroyed`
  (params (DestroyedActor :type "Actor Object Reference"))
  (`self.K2_DestroyActor`))

(fn `set_speed_arrow`
  (params (direction :type "Vector Structure"))
  (set `MovementComponent.Velocity` direction (`self.ProjectileMovement`)))

(fn `UserConstructionScript`)