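; Player bow weapon with a flipbook sprite, aimed and fired by mouse drag to launch arrow projectiles.
; Pressing after hovering its box starts the draw animation, which holds its last frame, while Tick rotates the bow from the drag offset.
; Release sets power from summed horizontal and vertical drag and fires the shoot event.
; If arrows remain, that event consumes one and spawns a projectile with item-based damage and drag-scaled velocity.
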(event `self.ReceiveBeginPlay`
  (add `self.shoot_event` (delegate `shoot_event_Event`))
  (`self.stop_shooting`))

(event `shoot_event_Event`
  (bind _com_my_arrow_short (`self.COM_my_arrow_short`))
  (if (> (`/Game/items/my_item_world/COM_my_arrow_short.my_arrow_count` _com_my_arrow_short) 0)
    (`/Game/items/my_item_world/COM_my_arrow_short.my_shoot_arrow` _com_my_arrow_short)
    (bind _returnvalue (`|SpawnActorFromClass` "/Game/BP_player/my_weapon_bow/my_projectile/BP_my_projectile_arrow.BP_my_projectile_arrow_C" (`SceneComponent.K2_GetComponentToWorld` (`self.animate_paper`)) "Undefined" "OverrideRootScale" null (`/Game/items/my_item_world/COM_my_item_property.value` (`self.COM_my_item_property`)) (`self.GetInstigator`)))
    (`/Game/BP_player/my_weapon_bow/my_projectile/BP_my_projectile_arrow.set_speed_arrow` _returnvalue (* (`SceneComponent.GetForwardVector` (`self.animate_paper`)) (`self.power_shoot`)))))

(event `self.animate_paper.OnFinishedPlaying`
  (bind _animate_paper (`self.animate_paper`))
  (`PaperFlipbookComponent.SetPlaybackPositionInFrames` _animate_paper (`PaperFlipbookComponent.GetFlipbookLengthInFrames` _animate_paper) false)
  (`PaperFlipbookComponent.SetLooping` _animate_paper false))

(event `self.ReceiveTick`
  (params (DeltaSeconds :type "Float (single-precision)"))
  (if (and (`PlayerController.bShowMouseCursor` (`GameplayStatics.GetPlayerController` 0)) (`self.is_ready_shoot`))
    (bind _returnvalue (`WidgetLayoutLibrary.GetMousePositionOnViewport`))
    (bind (_returnvalue_x _returnvalue_y) (`KismetMathLibrary.BreakVector2D` (- _returnvalue (`self.mouse_begin`))))
    (`SceneComponent.K2_SetRelativeRotation` (`self.animate_paper`) (`KismetMathLibrary.ComposeRotators` (`KismetMathLibrary.Conv_VectorToRotator` (`KismetMathLibrary.MakeVector` _returnvalue_y 0.0 _returnvalue_x)) (struct :`Pitch` 90.0)) false false)))

(event `self.Box.OnBeginCursorOver`
  (params (TouchedComponent :type "PrimitiveComponent Object Reference"))
  (if (not (`self.is_press_mouse`))
    (set `self.is_my_activate` true)))

(event `self.Box.OnEndCursorOver`
  (params (TouchedComponent :type "PrimitiveComponent Object Reference"))
  (if (not (`self.is_ready_shoot`))
    (set `self.is_my_activate` false)))

(fn `mouse_press`
  (returns (NewParam :type Boolean))
  (bind _animate_paper (`self.animate_paper`))
  (set `self.is_press_mouse` true)
  (if (and (`PlayerController.bShowMouseCursor` (`GameplayStatics.GetPlayerController` 0)) (`self.is_my_activate`))
    (bind _returnvalue (`WidgetLayoutLibrary.GetMousePositionOnViewport`))
    (set `self.mouse_begin` _returnvalue)
    (set `self.is_ready_shoot` true)
    (`SceneComponent.SetVisibility` (`self.MaterialBillboard`) false false)
    (`PaperFlipbookComponent.PlayFromStart` _animate_paper)
    (`GameplayStatics.PlaySoundAtLocation` "/Game/sound/bow/s_bow_spring_01.s_bow_spring_01" (`SceneComponent.K2_GetComponentLocation` _animate_paper) (struct) 1.0 1.0 0.0 null null null)))

(fn `mouse_realised`
  (returns (NewParam :type Boolean))
  (set `self.is_press_mouse` false)
  (if (and (`PlayerController.bShowMouseCursor` (`GameplayStatics.GetPlayerController` 0)) (`self.is_my_activate`))
    (bind _returnvalue (`WidgetLayoutLibrary.GetMousePositionOnViewport`))
    (bind (_returnvalue_x _returnvalue_y) (`KismetMathLibrary.BreakVector2D` (- (`self.mouse_begin`) _returnvalue)))
    (set `self.power_shoot` (+ (`KismetMathLibrary.Abs` _returnvalue_x) (`KismetMathLibrary.Abs` _returnvalue_y)))
    (`self.stop_shooting`)
    (`self.shoot_event`)
    (set `self.is_ready_shoot` false)
    (set `self.is_my_activate` false)
    (`GameplayStatics.PlaySoundAtLocation` "/Game/sound/bow/s_arrow_shoot_01.s_arrow_shoot_01" (`SceneComponent.K2_GetComponentLocation` (`self.animate_paper`)) (struct) 1.0 1.0 0.0 null null null)))

(fn `move_x`
  (params (x :type "Float (double-precision)"))
  (returns (NewParam :type Boolean))
  (return false))

(fn `move_y`
  (params (y :type "Float (double-precision)"))
  (returns (NewParam :type Boolean))
  (return false))

(fn `shoot_now`
  (`PaperFlipbookComponent.PlayFromStart` (`self.animate_paper`)))

(fn `stop_shooting`
  (bind _animate_paper (`self.animate_paper`))
  (`PaperFlipbookComponent.SetLooping` _animate_paper false)
  (`PaperFlipbookComponent.Stop` _animate_paper)
  (`PaperFlipbookComponent.SetPlaybackPositionInFrames` _animate_paper 0 false))

(fn `UserConstructionScript`)