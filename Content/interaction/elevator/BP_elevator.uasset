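; Elevator actor that shuttles its Collider back and forth between two points, PosA and PosB, set relative to its starting location.
; BeginPlay converts both offsets to world space and derives velocities from their separation times Speed, so travel time is independent of distance.
; While IsTime and ElevatorLoop are true, Tick moves the Collider without sweep until every axis is within StopElevator of the target.
; Arrival flips direction and pauses movement until a short timer calls time_stop.
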(event `self.ReceiveBeginPlay`
  (bind _pos_a (`self.pos_a`))
  (bind _pos_b (`self.pos_b`))
  (bind _returnvalue (`SceneComponent.K2_GetComponentLocation` (`self.collider`)))
  (set `self.pos_a` (+ _returnvalue (`self.pos_a`)))
  (set `self.pos_b` (+ _returnvalue (`self.pos_b`)))
  (set `self.pos_speed_a` (* (- _pos_a _pos_b) (`self.speed`)))
  (set `self.pos_speed_b` (* (- _pos_b _pos_a) (`self.speed`))))

(event `self.ReceiveTick`
  (params (DeltaSeconds :type "Float (single-precision)"))
  (bind _collider (`self.collider`))
  (bind _stop_elevator (`self.stop_elevator`))
  (bind _collider_2 (`self.collider`))
  (bind _stop_elevator_2 (`self.stop_elevator`))
  (bind (_returnvalue_x _returnvalue_y _returnvalue_z) (`KismetMathLibrary.BreakVector` (- (`SceneComponent.K2_GetComponentLocation` _collider_2) (`self.pos_b`))))
  (bind (_returnvalue_x_2 _returnvalue_y_2 _returnvalue_z_2) (`KismetMathLibrary.BreakVector` (- (`SceneComponent.K2_GetComponentLocation` _collider) (`self.pos_a`))))
  (if (`self.is_time`)
    (if (`self.elevator_loop`)
      (if (`self.is_go_up`)
        (`SceneComponent.K2_AddWorldOffset` _collider (* (`self.pos_speed_a`) (`GameplayStatics.GetWorldDeltaSeconds`)) false false)
        (if (and (< (`KismetMathLibrary.Abs` _returnvalue_x_2) _stop_elevator) (< (`KismetMathLibrary.Abs` _returnvalue_y_2) _stop_elevator) (< (`KismetMathLibrary.Abs` _returnvalue_z_2) _stop_elevator))
          (`self.even_el_stop`))
        (else
          (`SceneComponent.K2_AddWorldOffset` _collider_2 (* (`self.pos_speed_b`) (`GameplayStatics.GetWorldDeltaSeconds`)) false false)
          (if (and (< (`KismetMathLibrary.Abs` _returnvalue_x) _stop_elevator_2) (< (`KismetMathLibrary.Abs` _returnvalue_y) _stop_elevator_2) (< (`KismetMathLibrary.Abs` _returnvalue_z) _stop_elevator_2))
            (`self.even_el_stop`)))))))

(event `even_el_stop`
  (set `self.is_go_up` (not (`self.is_go_up`)))
  (set `self.is_time` false)
  (`KismetSystemLibrary.K2_SetTimer` null "time_stop" 1.5))

(fn `time_stop`
  (set `self.is_time` true))

(fn `UserConstructionScript`)