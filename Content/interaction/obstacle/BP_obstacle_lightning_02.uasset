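; Paper2D lightning obstacle that repeatedly strikes on a timer and damages actors that touch it.
; After a start delay it shows and plays a non-looping flipbook, plays a thunder sound and enables query-only collision.
; When the flipbook finishes, it hides, disables collision and schedules the next strike after a pause.
; Overlapping actors take fixed damage using a custom damage type.
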(event `self.ReceiveBeginPlay`
  (`PaperFlipbookComponent.Stop` (`self.PaperFlipbook`))
  (`PaperFlipbookComponent.SetLooping` (`self.PaperFlipbook`) false)
  (`SceneComponent.SetVisibility` (`self.PaperFlipbook`) false true)
  (`KismetSystemLibrary.K2_SetTimer` null "my_play_start" (`self.start_dalay`)))

(event `self.PaperFlipbook.OnFinishedPlaying`
  (`self.my_play_end`))

(event `self.collision.OnComponentBeginOverlap`
  (params (OverlappedComponent :type "PrimitiveComponent Object Reference") (OtherActor :type "Actor Object Reference") (OtherComp :type "PrimitiveComponent Object Reference") (OtherBodyIndex :type Integer) (bFromSweep :type Boolean) (SweepResult :type "HitResult Structure (by ref)"))
  (`GameplayStatics.ApplyDamage` OtherActor 11.0 null self "/Game/interaction/barrel_explode/BP_my_dame_type.BP_my_dame_type_C"))

(fn `my_play_end`
  (`SceneComponent.SetVisibility` (`self.PaperFlipbook`) false true)
  (`KismetSystemLibrary.K2_SetTimer` null "my_play_start" (`self.beetwen_animation`))
  (`PrimitiveComponent.SetCollisionEnabled` (`self.collision`) "NoCollision"))

(fn `my_play_start`
  (`SceneComponent.SetVisibility` (`self.PaperFlipbook`) true true)
  (`PaperFlipbookComponent.PlayFromStart` (`self.PaperFlipbook`))
  (`PrimitiveComponent.SetCollisionEnabled` (`self.collision`) "QueryOnly")
  (`GameplayStatics.PlaySoundAtLocation` "/Game/sound/lightning/S_my_lightning.S_my_lightning" (`SceneComponent.K2_GetComponentLocation` (`self.PaperFlipbook`)) (struct) 1.0 1.0 0.0 null null null))

(fn `UserConstructionScript`)