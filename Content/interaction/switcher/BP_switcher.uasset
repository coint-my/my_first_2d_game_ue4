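; BP_switcher is a player-usable switch that toggles its sprite and the looping of a linked elevator.
; Overlapping its Interact component binds an event to the paper player's use action, and leaving unbinds it.
; CheckCanOpenEndClose picks MyOpen or MyClose while active, with IsOpen holding the inverse of the switch's state.
; Opening also clears IsActivate, so later checks only print a deactivated message unless it is re-enabled.
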(event `self.ReceiveBeginPlay`
  (`self.my_close`))

(event `self.interact.OnComponentBeginOverlap`
  (params (OverlappedComponent :type "PrimitiveComponent Object Reference") (OtherActor :type "Actor Object Reference") (OtherComp :type "PrimitiveComponent Object Reference") (OtherBodyIndex :type Integer) (bFromSweep :type Boolean) (SweepResult :type "HitResult Structure (by ref)"))
  (bind _ascharacter_paper_player (cast `/Game/BP_player/character_paper_player` OtherActor))
  (add `/Game/BP_player/character_paper_player.use_player` _ascharacter_paper_player (`|CreateDelegate` :!event `check_can_open_end_close`)))

(event `self.interact.OnComponentEndOverlap`
  (params (OverlappedComponent :type "PrimitiveComponent Object Reference") (OtherActor :type "Actor Object Reference") (OtherComp :type "PrimitiveComponent Object Reference") (OtherBodyIndex :type Integer))
  (bind _ascharacter_paper_player (cast `/Game/BP_player/character_paper_player` OtherActor))
  (remove `/Game/BP_player/character_paper_player.use_player` _ascharacter_paper_player (`|CreateDelegate` :!event `check_can_open_end_close`)))

(fn `check_can_open_end_close`
  (if (`self.is_activate`)
    (if (`self.is_open`)
      (bind _val (`self.my_open`))
      (bind _output_get (set `self.is_open` (not _val)))
      (set `self.is_activate` _output_get)
      (else
        (bind _val_2 (`self.my_close`))
        (set `self.is_open` (not _val_2))))
    (else
      (`KismetSystemLibrary.PrintString` "this is deactivated"))))

(fn `my_close`
  (returns (val :type Boolean))
  (`PaperSpriteComponent.SetSprite` (`self.sprite`) "/Game/spraites/texture/setting_level_05/S_switcher_close.S_switcher_close")
  (set `/Game/interaction/elevator/BP_elevator.elevator_loop` false (`self.my_elevator`))
  (return false))

(fn `my_open`
  (returns (val :type Boolean))
  (`PaperSpriteComponent.SetSprite` (`self.sprite`) "/Game/spraites/texture/setting_level_05/S_switcher_open.S_switcher_open")
  (set `/Game/interaction/elevator/BP_elevator.elevator_loop` true (`self.my_elevator`))
  (return true))

(fn `UserConstructionScript`
  (bind _val (`self.my_close`))
  (set `self.is_open` (not _val)))