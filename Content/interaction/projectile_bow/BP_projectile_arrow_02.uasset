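; Arrow projectile for the bow that flies a parabolic arc in the XZ plane, damaging or sticking to what it hits.
; AddVelosity stores launch velocity, start position and gravity, and a fast looping timer increments a counter that TestParabola uses to compute position and face along the path, without physics simulation.
; Overlapping a damageable actor deals damage scaled by horizontal launch speed and destroys the arrow; otherwise it stops, attaches and plays a sound.
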(event `self.ReceiveBeginPlay`
  (`KismetSystemLibrary.K2_SetTimer` null "count_time" 0.01 true))

(event `self.ReceiveActorBeginOverlap`
  (params (OtherActor :type "Actor Object Reference"))
  (bind _velocity_x (`KismetMathLibrary.BreakVector` (`self.velocity`)))
  (if (`self.is_stop`)
    _
    (elif (`Actor.bCanBeDamaged` OtherActor)
      (`GameplayStatics.ApplyDamage` OtherActor (`KismetMathLibrary.Conv_IntToDouble` (`KismetMathLibrary.Max` (`KismetMathLibrary.Round` (`KismetMathLibrary.Abs` _velocity_x)) 1)))
      (`self.K2_DestroyActor`)
      (else
        (`KismetSystemLibrary.K2_ClearTimer` null "count_time")
        (`self.K2_AttachToActor` self OtherActor "None" "KeepWorld" "KeepWorld" "KeepWorld" true)
        (set `self.is_stop` true)
        (`GameplayStatics.PlaySound2D` "/Game/sound/bow/s_arrow_end.s_arrow_end" 1.0 1.0 0.0 null null)))))

(fn `add_velosity`
  (params (velocity :type "Vector Structure") (start_pos :type "Vector Structure") (gravity :type "Float (double-precision)"))
  (set `self.velocity` velocity)
  (set `self.start_position` start_pos)
  (set `self.gravity` gravity))

(fn `count_time`
  (`/Engine/EditorBlueprintResources/StandardMacros.IncrementFloat` (`self.counter`)
    (:`  `
      (`self.test_parabola` (`self.velocity`) (`self.start_position`)))))

(fn `test_parabola`
  (params (velocity :type "Vector Structure") (start_pos :type "Vector Structure"))
  (bind _counter (`self.counter`))
  (bind (_old_position_x _old_position_y _old_position_z) (`KismetMathLibrary.BreakVector` (`self.old_position`)))
  (bind (_returnvalue_x _returnvalue_y _returnvalue_z) (`KismetMathLibrary.BreakVector` (* velocity _counter)))
  (bind _returnvalue (+ start_pos_X _returnvalue_x))
  (bind _returnvalue_2 (- (+ start_pos_Z _returnvalue_z) (* (* _counter _counter) (`self.gravity`))))
  (`self.K2_SetActorRelativeLocation` (`KismetMathLibrary.MakeVector` _returnvalue 0.0 _returnvalue_2))
  (`self.K2_SetActorRotation` (`KismetMathLibrary.FindLookAtRotation` (`KismetMathLibrary.MakeVector` _old_position_x 0.0 _old_position_z) (`KismetMathLibrary.MakeVector` _returnvalue 0.0 _returnvalue_2)))
  (set `self.old_position` (`KismetMathLibrary.MakeVector` _returnvalue 0.0 _returnvalue_2)))

(fn `UserConstructionScript`)