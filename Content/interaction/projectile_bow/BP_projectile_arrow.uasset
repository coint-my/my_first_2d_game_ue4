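; Arrow projectile for the bow that flies under physics and damages what its point hits.
; SetShootForce launches it with a forward impulse on SpArrow, applied at the PointPos location.
; Overlapping a damageable actor with Point_damage deals damage scaled by mass and summed X and Z velocity, ignoring Y, then destroys the arrow.
; The arrow also destroys itself once TimeAlive expires.
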(event `self.ReceiveBeginPlay`
  (`KismetSystemLibrary.Delay` (`self.time_alive`))
  (`self.K2_DestroyActor`))

(event `self.point_damage.OnComponentBeginOverlap`
  (params (OverlappedComponent :type "PrimitiveComponent Object Reference") (OtherActor :type "Actor Object Reference") (OtherComp :type "PrimitiveComponent Object Reference") (OtherBodyIndex :type Integer) (bFromSweep :type Boolean) (SweepResult :type "HitResult Structure (by ref)"))
  (bind _sp_arrow (`self.sp_arrow`))
  (bind _returnvalue (`PrimitiveComponent.GetPhysicsLinearVelocity` _sp_arrow "None"))
  (if (`Actor.bCanBeDamaged` OtherActor)
    (`GameplayStatics.ApplyDamage` OtherActor (`KismetMathLibrary.Conv_IntToDouble` (`KismetMathLibrary.Abs_Int` (`KismetMathLibrary.Round` (/ (* (+ (.z _returnvalue) (.x _returnvalue)) (`PrimitiveComponent.GetMass` _sp_arrow)) 1000.0)))))
    (`self.K2_DestroyActor`)))

(fn `set_shoot_force`
  (params (force :type "Float (double-precision)"))
  (bind _sp_arrow (`self.sp_arrow`))
  (`PrimitiveComponent.AddImpulseAtLocation` _sp_arrow (* (`SceneComponent.GetForwardVector` _sp_arrow) force) (`SceneComponent.K2_GetComponentLocation` (`self.point_pos`)) "None"))

(fn `UserConstructionScript`)