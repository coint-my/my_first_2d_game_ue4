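; BP_Bow_03 is a projectile bow test actor that previews a parabolic arc toward the player.
; Every tick it moves point 1 of the LineParabola spline to player 0's location and sets a fixed local tangent to bend the curve.
; It then samples the spline at Loop evenly spaced times and draws white debug points along it, with no projectile spawning or firing logic.
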(event `self.ReceiveBeginPlay`)

(event `self.ReceiveTick`
  (params (DeltaSeconds :type "Float (single-precision)"))
  (`self.test_parabola`))

(fn `test_parabola`
  (bind _line_parabola (`self.line_parabola`))
  (`SplineComponent.SetLocationAtSplinePoint` _line_parabola 1 (`self.K2_GetActorLocation` (`GameplayStatics.GetPlayerCharacter` 0)) "World" true)
  (`SplineComponent.SetTangentAtSplinePoint` _line_parabola 0 (-400.0 0.0 400.0) "Local" true)
  (for _index (range 1 (+ (`self.loop`) 1))
    (`KismetSystemLibrary.DrawDebugPoint` (`SplineComponent.GetLocationAtTime` (`self.line_parabola`) (/ (`KismetMathLibrary.Conv_IntToDouble` _index) (`KismetMathLibrary.Conv_IntToDouble` (`self.loop`))) "World" false) 10.0 (struct :`R` 1.0 :`G` 1.0 :`B` 1.0 :`A` 1.0))))

(fn `UserConstructionScript`)