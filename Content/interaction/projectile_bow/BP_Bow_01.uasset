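; BP_Bow_01 is a flipbook-based bow that turns toward the player and fires arrow projectiles.
; Every tick it aims the flipbook at player 0, adjusting pitch from the square root of the X distance, and draws a debug line.
; Shoot plays the animation if reloaded; when it finishes, an arrow spawns with the configured force and the bow re-arms.
; An uncalled TestParabola helper plots a quadratic arc with debug points.
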(event `self.ReceiveBeginPlay`
  (bind _fb_bow (`self.fb_bow`))
  (`PaperFlipbookComponent.SetLooping` _fb_bow false)
  (`PaperFlipbookComponent.Stop` _fb_bow)
  (`PaperFlipbookComponent.SetPlaybackPositionInFrames` _fb_bow 0 false)
  (`PaperFlipbookComponent.SetPlayRate` _fb_bow (`self.speed_reload`)))

(event `self.ReceiveTick`
  (params (DeltaSeconds :type "Float (single-precision)"))
  (`self.initialize_trajectory`))

(event `self.fb_bow.OnFinishedPlaying`
  (bind _fb_bow (`self.fb_bow`))
  (`PaperFlipbookComponent.SetPlaybackPositionInFrames` (`self.fb_bow`) 0 false)
  (bind _returnvalue (`|SpawnActorFromClass` "/Game/interaction/projectile_bow/BP_projectile_arrow.BP_projectile_arrow_C" (`KismetMathLibrary.MakeTransform` (`SceneComponent.K2_GetComponentLocation` _fb_bow) (`SceneComponent.K2_GetComponentRotation` _fb_bow)) "Undefined" "OverrideRootScale" null null))
  (`/Game/interaction/projectile_bow/BP_projectile_arrow.set_shoot_force` _returnvalue (`self.arrow_force`))
  (set `self.is_flag_reload` true))

(fn `initialize_trajectory`
  (locals (dist :type "Float (double-precision)"))
  (bind _returnvalue (`GameplayStatics.GetPlayerCharacter` 0))
  (bind _fb_bow (`self.fb_bow`))
  (bind _start_end_point (make `/Game/interaction/projectile_bow/start_end_point` (`self.K2_GetActorLocation` self) (`self.K2_GetActorLocation` _returnvalue)))
  (bind (_start _end) (break `/Game/interaction/projectile_bow/start_end_point` _start_end_point))
  (bind (_start_2 _end_2) (break `/Game/interaction/projectile_bow/start_end_point` _start_end_point))
  (set `local.dist` (`self.GetDistanceTo` _returnvalue self))
  (bind _result (`/Engine/EditorBlueprintResources/StandardMacros.NegateFloat` (`KismetMathLibrary.Sqrt` (`KismetMathLibrary.Abs` (- (.x _start_2) (.x _end_2)))))
    (:`  `
      (`SceneComponent.K2_SetWorldRotation` _fb_bow (`KismetMathLibrary.NormalizedDeltaRotator` (`KismetMathLibrary.FindLookAtRotation` (`SceneComponent.K2_GetComponentLocation` _fb_bow) (`self.K2_GetActorLocation` _returnvalue)) (`KismetMathLibrary.MakeRotator` 0.0 _result)) false false)
      (`KismetSystemLibrary.DrawDebugLine` _start _end (struct :`R` 0.382848 :`G` 0.578125 :`B` 0.210577 :`A` 1.0)))))

(fn `shoot`
  (if (`self.is_flag_reload`)
    (`PaperFlipbookComponent.PlayFromStart` (`self.fb_bow`))
    (set `self.is_flag_reload` false)))

(fn `test_parabola`
  (params (points :type "/Game/interaction/projectile_bow/start_end_point Structure"))
  (locals (a :type "Float (double-precision)" :default 0.0003) (b :type "Float (double-precision)" :default 0.1) (c :type "Float (double-precision)" :default 0.0) (loop :type Integer :default 100) (x1 :type "Float (double-precision)") (z1 :type "Float (double-precision)") (x_pre :type "Float (double-precision)") (z_pre :type "Float (double-precision)"))
  (bind _x1 (`local.x1`))
  (bind (_returnvalue_x _returnvalue_y _returnvalue_z) (`KismetMathLibrary.BreakVector` (`SceneComponent.K2_GetComponentLocation` (`self.fb_bow`))))
  (for _index (range (+ (`local.loop`) 1))
    (bind _output_get (set `local.x1` (`KismetMathLibrary.Conv_IntToDouble` _index)))
    (bind _output_get_2 (set `local.z1` (+ (* (`local.a`) (* _x1 _x1)) (+ (* (`local.b`) (`local.x1`)) (`local.c`)))))
    (bind _output_get_3 (set `local.x1` (+ _returnvalue_x _output_get)))
    (bind _output_get_4 (set `local.z1` (- _returnvalue_z _output_get_2)))
    (`KismetSystemLibrary.DrawDebugPoint` (`KismetMathLibrary.MakeVector` _output_get_3 0.0 _output_get_4) 2.0 (struct :`R` 0.113357 :`G` 1.0 :`A` 1.0))))

(fn `UserConstructionScript`)