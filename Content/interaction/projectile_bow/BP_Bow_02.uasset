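; Automated 2D bow enemy that aims at the player and fires ballistic arrows.
; While Radius_range is overlapped, each tick tilts the bow with a heuristic arc offset and steps the Intersect component along the predicted parabola, drawing debug points.
; Intersect overlaps flag whether the player is hit, and a looping timer shoots when flagged and reloaded.
; The finished flipbook animation spawns BP_projectile_arrow_02 with the computed velocity and gravity, then re-arms the bow.
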(event `self.ReceiveBeginPlay`
  (bind _flip_bow_02 (`self.flip_bow_02`))
  (`PaperFlipbookComponent.SetLooping` _flip_bow_02 false)
  (`PaperFlipbookComponent.Stop` _flip_bow_02)
  (`PaperFlipbookComponent.SetPlaybackPositionInFrames` _flip_bow_02 0 false)
  (`PaperFlipbookComponent.SetPlayRate` _flip_bow_02 (`self.anim_speed`))
  (set `self.is_flag_reload` true)
  (`KismetSystemLibrary.K2_SetTimer` null "look_from_fire" (`self.time_spawn_fire`) true))

(event `self.ReceiveTick`
  (params (DeltaSeconds :type "Float (single-precision)"))
  (if (`self.is_radius_range`)
    (`self.test_parabola` DeltaSeconds)))

(event `self.flip_bow_02.OnFinishedPlaying`
  (bind _flip_bow_02 (`self.flip_bow_02`))
  (bind _returnvalue (`SceneComponent.K2_GetComponentLocation` _flip_bow_02))
  (`PaperFlipbookComponent.SetPlaybackPositionInFrames` (`self.flip_bow_02`) 0 false)
  (bind _returnvalue_2 (`|SpawnActorFromClass` "/Game/interaction/projectile_bow/BP_projectile_arrow_02.BP_projectile_arrow_02_C" (`KismetMathLibrary.MakeTransform` _returnvalue (`SceneComponent.K2_GetComponentRotation` _flip_bow_02)) "Undefined" "OverrideRootScale" null null))
  (`/Game/interaction/projectile_bow/BP_projectile_arrow_02.add_velosity` _returnvalue_2 (`self.velocity`) _returnvalue (`self.gravity`))
  (set `self.is_flag_reload` true))

(event `self.intersect.OnComponentBeginOverlap`
  (params (OverlappedComponent :type "PrimitiveComponent Object Reference") (OtherActor :type "Actor Object Reference") (OtherComp :type "PrimitiveComponent Object Reference") (OtherBodyIndex :type Integer) (bFromSweep :type Boolean) (SweepResult :type "HitResult Structure (by ref)"))
  (set `self.is_intersect` true)
  (cast `/Game/BP_player/character_paper_player` OtherActor
    (:`then`
      (set `self.is_enemy_unit` true))
    (:`CastFailed`
      (set `self.is_enemy_unit` false))))

(event `self.radius_range.OnComponentBeginOverlap`
  (params (OverlappedComponent :type "PrimitiveComponent Object Reference") (OtherActor :type "Actor Object Reference") (OtherComp :type "PrimitiveComponent Object Reference") (OtherBodyIndex :type Integer) (bFromSweep :type Boolean) (SweepResult :type "HitResult Structure (by ref)"))
  (set `self.is_radius_range` true))

(event `self.radius_range.OnComponentEndOverlap`
  (params (OverlappedComponent :type "PrimitiveComponent Object Reference") (OtherActor :type "Actor Object Reference") (OtherComp :type "PrimitiveComponent Object Reference") (OtherBodyIndex :type Integer))
  (set `self.is_radius_range` false)
  (set `self.is_enemy_unit` false))

(fn `look_from_fire`
  (if (`self.is_enemy_unit`)
    (`self.shoot`)))

(fn `rotation_bow`
  (locals (if_mid :type "Float (double-precision)"))
  (bind _returnvalue (`GameplayStatics.GetPlayerCharacter` 0))
  (bind (_returnvalue_x _returnvalue_y _returnvalue_z) (`KismetMathLibrary.BreakVector` (`self.K2_GetActorLocation` _returnvalue)))
  (bind (_returnvalue_x_2 _returnvalue_y_2 _returnvalue_z_2) (`KismetMathLibrary.BreakVector` (`self.K2_GetActorLocation` self)))
  (bind _returnvalue_2 (* (- _returnvalue_x _returnvalue_x_2) (* (`self.gravity`) 1.25)))
  (bind _returnvalue_3 (`KismetMathLibrary.Sqrt` (* _returnvalue_2 _returnvalue_2)))
  (if (< _returnvalue_3 12.0)
    (set `local.if_mid` 0.0)
    (else
      (set `local.if_mid` (* (`KismetMathLibrary.Sqrt` (- _returnvalue_z_2 _returnvalue_z)) 0.4))))
  (`self.K2_SetActorRotation` (`KismetMathLibrary.NormalizedDeltaRotator` (`KismetMathLibrary.FindLookAtRotation` (`self.K2_GetActorLocation` _returnvalue) (`self.K2_GetActorLocation` self)) (`KismetMathLibrary.MakeRotator` 0.0 (- (- _returnvalue_3 (`local.if_mid`)) 180.0)))))

(fn `shoot`
  (if (`self.is_flag_reload`)
    (`PaperFlipbookComponent.PlayFromStart` (`self.flip_bow_02`))
    (set `self.is_flag_reload` false)
    (`GameplayStatics.PlaySound2D` "/Game/sound/bow/s_arrow_begin.s_arrow_begin" 1.0 1.0 0.0 null null)))

(fn `test_parabola`
  (params (time :type "Float (double-precision)"))
  (locals (old_pos :type "Vector Structure") (if_mid :type "Float (double-precision)"))
  (bind (_returnvalue_x _returnvalue_y _returnvalue_z) (`KismetMathLibrary.BreakVector` (`self.K2_GetActorLocation`)))
  (set `self.velocity` (* (`SceneComponent.GetForwardVector` (`self.flip_bow_02`)) (`self.speed`)))
  (set `self.is_intersect` false)
  (`self.rotation_bow`)
  (for _index (range (+ (`self.loop`) 1))
    (bind (_returnvalue_x_2 _returnvalue_y_2 _returnvalue_z_2) (`KismetMathLibrary.BreakVector` (* (`self.velocity`) _index)))
    (bind _returnvalue (+ _returnvalue_x _returnvalue_x_2))
    (bind _returnvalue_2 (- (+ _returnvalue_z _returnvalue_z_2) (* (* _index (`KismetMathLibrary.Conv_IntToDouble` _index)) (`self.gravity`))))
    (`SceneComponent.K2_SetWorldLocation` (`self.intersect`) (`KismetMathLibrary.MakeVector` _returnvalue 0.0 _returnvalue_2) false false)
    (if (`self.is_intersect`)
      (return)
      (else
        (`KismetSystemLibrary.DrawDebugPoint` (`KismetMathLibrary.MakeVector` _returnvalue 0.0 _returnvalue_2) 3.0 (struct :`R` 0.113357 :`G` 1.0 :`A` 1.0))))))

(fn `UserConstructionScript`)