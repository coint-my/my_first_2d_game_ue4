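; Fire effect actor, apparently for an exploding barrel, that plays an explosion sound on spawn and damages an actor inside its Box.
; Box overlaps track one actor, clearing it on any end overlap.
; Tick uses a Delay to throttle custom-typed damage to roughly five hits per second.
; Tick also traces below the Capsule until it hits WorldStatic, then disables physics and collision so the fire settles.
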(event `self.ReceiveBeginPlay`
  (`GameplayStatics.PlaySoundAtLocation` "/Game/sound/explode/S_my_explode.S_my_explode" (`SceneComponent.K2_GetComponentLocation` (`self.Capsule`)) (struct) 1.0 1.0 0.0 null null null))

(event `self.ReceiveTick`
  (params (DeltaSeconds :type "Float (single-precision)"))
  (bind _capsule (`self.Capsule`))
  (bind _temp_actor (`self.temp_actor`))
  (bind _returnvalue (`SceneComponent.K2_GetComponentLocation` (`self.Capsule`)))
  (`|ExecutionSequence`
    (:`then_0`
      (if (`self.is_trigger`)
        (`KismetSystemLibrary.Delay` 0.2)
        (`/Engine/EditorBlueprintResources/StandardMacros.IsValid` _temp_actor
          (:`Is Valid`
            (`GameplayStatics.ApplyDamage` _temp_actor (`self.my_damage`) null self "/Game/interaction/barrel_explode/BP_my_dame_type.BP_my_dame_type_C")))))
    (:`then_1`
      (if (not (`self.is_test_hit`))
        (bind (_outhit _returnvalue_2) (`KismetSystemLibrary.LineTraceSingleForObjects` _returnvalue (+ _returnvalue (* (`KismetMathLibrary.NegateVector` (`self.GetActorUpVector`)) 20.0)) (`|MakeArray` "ObjectTypeQuery1" :!type "EObjectTypeQuery Enum")))
        (bind _output_get (set `self.is_test_hit` _returnvalue_2))
        (if _output_get
          (`PrimitiveComponent.SetSimulatePhysics` _capsule false)
          (`PrimitiveComponent.SetCollisionEnabled` _capsule "NoCollision"))))))

(event `self.Box.OnComponentBeginOverlap`
  (params (OverlappedComponent :type "PrimitiveComponent Object Reference") (OtherActor :type "Actor Object Reference") (OtherComp :type "PrimitiveComponent Object Reference") (OtherBodyIndex :type Integer) (bFromSweep :type Boolean) (SweepResult :type "HitResult Structure (by ref)"))
  (set `self.is_trigger` true)
  (`/Engine/EditorBlueprintResources/StandardMacros.IsValid` (`self.temp_actor`)
    (:`Is Not Valid`
      (set `self.temp_actor` OtherActor))))

(event `self.Box.OnComponentEndOverlap`
  (params (OverlappedComponent :type "PrimitiveComponent Object Reference") (OtherActor :type "Actor Object Reference") (OtherComp :type "PrimitiveComponent Object Reference") (OtherBodyIndex :type Integer))
  (set `self.is_trigger` false)
  (set `self.temp_actor` null))

(fn `UserConstructionScript`)