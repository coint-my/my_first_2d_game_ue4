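; BP_barrel_explode is an explosive barrel that blows up when its explosion collider overlaps something while its vertical velocity is below the PicExplode threshold.
; The overlap starts a short timer that calls on_explode.
; That function spawns a fire effect actor with a quarter of the item property's damage, applies full radial damage using the RadialForce radius, emits sparks and destroys the barrel.
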(event `self.collider_explode.OnComponentBeginOverlap`
  (params (OverlappedComponent :type "PrimitiveComponent Object Reference") (OtherActor :type "Actor Object Reference") (OtherComp :type "PrimitiveComponent Object Reference") (OtherBodyIndex :type Integer) (bFromSweep :type Boolean) (SweepResult :type "HitResult Structure (by ref)"))
  (bind (_returnvalue_x _returnvalue_y _returnvalue_z) (`KismetMathLibrary.BreakVector` (`self.GetVelocity`)))
  (if (< _returnvalue_z (`self.pic_explode`))
    (`KismetSystemLibrary.K2_SetTimer` null "on_explode" 0.5)))

(fn `on_explode`
  (`|SpawnActorFromClass` "/Game/interaction/barrel_explode/BP_my_effect_fire.BP_my_effect_fire_C" (`self.GetTransform`) "Undefined" "OverrideRootScale" null (/ (`/Game/items/my_item_world/COM_my_item_property.value` (`self.COM_my_item_property`)) 4.0) null)
  (`KismetSystemLibrary.K2_ClearTimer` null "on_explode")
  (`GameplayStatics.ApplyRadialDamage` :`BaseDamage` (`/Game/items/my_item_world/COM_my_item_property.value` (`self.COM_my_item_property`)) :`Origin` (`self.K2_GetActorLocation`) :`DamageRadius` (`RadialForceComponent.Radius` (`self.RadialForce`)) :`DamageTypeClass` "/Game/interaction/barrel_explode/BP_my_dame_type.BP_my_dame_type_C" :`DamageCauser` self :`InstigatedByController` (`AIBlueprintHelperLibrary.GetAIController` self))
  (`GameplayStatics.SpawnEmitterAtLocation` "/Game/particle/sparks/P_my_spark_01.P_my_spark_01" (`self.K2_GetActorLocation`))
  (`self.K2_DestroyActor`))

(fn `UserConstructionScript`)