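; Trampoline actor that bounces the paper player character back up when it falls onto the collider.
; Any downward-moving overlap plays the animation once; only the player also gets the bounce and a 2D sound.
; The upward impulse is twice the fall speed as a mass-independent velocity change, effectively reversing the vertical velocity.
; An IsFinished flag is set when the animation ends but is not read in this graph.
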(event `self.ReceiveBeginPlay`
  (`PaperFlipbookComponent.SetLooping` (`self.animate`) false)
  (set `self.is_finished` false))

(event `self.animate.OnFinishedPlaying`
  (set `self.is_finished` true)
  (`PaperFlipbookComponent.SetLooping` (`self.animate`) false))

(event `self.collider.OnComponentBeginOverlap`
  (params (OverlappedComponent :type "PrimitiveComponent Object Reference") (OtherActor :type "Actor Object Reference") (OtherComp :type "PrimitiveComponent Object Reference") (OtherBodyIndex :type Integer) (bFromSweep :type Boolean) (SweepResult :type "HitResult Structure (by ref)"))
  (bind (_returnvalue_x _returnvalue_y _returnvalue_z) (`KismetMathLibrary.BreakVector` (`self.GetVelocity` OtherActor)))
  (if (< _returnvalue_z 0.0)
    (`PaperFlipbookComponent.PlayFromStart` (`self.animate`))
    (bind _ascharacter_paper_player (cast `/Game/BP_player/character_paper_player` OtherActor))
    (`CharacterMovementComponent.AddImpulse` (`Character.CharacterMovement` _ascharacter_paper_player) (`KismetMathLibrary.MakeVector` 0.0 0.0 (* (`KismetMathLibrary.Abs` _returnvalue_z) 2.0)) true)
    (`GameplayStatics.PlaySound2D` "/Game/sound/trampoline_sound/trampoline_sound.trampoline_sound" 1.0 1.0 0.0 null null)))

(fn `UserConstructionScript`)