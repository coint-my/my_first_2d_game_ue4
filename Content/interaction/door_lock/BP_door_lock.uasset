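; Door lock actor that shows a colored lock sprite and prompts the player with the use key; no unlock logic is in this graph.
; The construction script picks the sprite from ColorKey.
; A box overlap writes the key bound to the "use" action into the info_door_lock widget and calls FalloffText(true).
; A name-based timer later calls reset_info, which calls FalloffText(false).
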(event `self.Box.OnComponentBeginOverlap`
  (params (OverlappedComponent :type "PrimitiveComponent Object Reference") (OtherActor :type "Actor Object Reference") (OtherComp :type "PrimitiveComponent Object Reference") (OtherBodyIndex :type Integer) (bFromSweep :type Boolean) (SweepResult :type "HitResult Structure (by ref)"))
  (`self.info_press`))

(fn `info_press`
  (bind _asinfo_door_lock (cast `/Game/interaction/door_lock/info_door_lock` (`WidgetComponent.GetUserWidgetObject` (`self.widget_info`))))
  (`Widget.SetVisibility` _asinfo_door_lock "Visible")
  (`/Game/interaction/door_lock/info_door_lock.set_text` _asinfo_door_lock (`KismetStringLibrary.Concat_StrStr` "press key(" (`KismetTextLibrary.Conv_TextToString` (`KismetInputLibrary.Key_GetDisplayName` (`.Key` (break `InputActionKeyMapping` (`|GetArrayItem` (`InputSettings.GetActionMappingByName` (`InputSettings.GetInputSettings`) "use")))))) ")"))
  (`/Game/interaction/door_lock/info_door_lock.falloff_text` _asinfo_door_lock true)
  (`KismetSystemLibrary.K2_SetTimer` null "reset_info" 4.0))

(fn `reset_info`
  (bind _asinfo_door_lock (cast `/Game/interaction/door_lock/info_door_lock` (`WidgetComponent.GetUserWidgetObject` (`self.widget_info`))))
  (`/Game/interaction/door_lock/info_door_lock.falloff_text` _asinfo_door_lock false))

(fn `UserConstructionScript`
  (`PaperSpriteComponent.SetSprite` (`self.sprite`) (select `/Game/my_enum/E_color_key` (`self.color_key`) :`NewEnumerator0` "/Game/spraites/texture/setting_level/door_lock_red.door_lock_red" :`NewEnumerator1` "/Game/spraites/texture/setting_level/door_lock_green.door_lock_green" :`NewEnumerator2` "/Game/spraites/texture/setting_level/dor_lock_yellow.dor_lock_yellow" :`NewEnumerator3` "/Game/spraites/texture/setting_level/door_lock_blue.door_lock_blue" :!type "PaperSprite Object Reference")))