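; Interactable info table that shows its configured text in a widget when a nearby player presses use.
; Collider overlap binds and unbinds the player's use event; leaving also hides the text.
; On entry, a second widget, reusing the info_door_lock class, shows a key prompt built from the "use" input mapping, with its falloff switched off by a timer.
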(event `self.ReceiveBeginPlay`
  (bind _asinfo_table (cast `/Game/UI/info_table` (`WidgetComponent.GetUserWidgetObject` (`self.widget_text`))))
  (bind _output_get (set `self.w_text` _asinfo_table))
  (`/Game/UI/info_table.set_text_info` _output_get (`self.text_info`))
  (`Widget.SetVisibility` _output_get "Hidden"))

(event `self.collider.OnComponentBeginOverlap`
  (params (OverlappedComponent :type "PrimitiveComponent Object Reference") (OtherActor :type "Actor Object Reference") (OtherComp :type "PrimitiveComponent Object Reference") (OtherBodyIndex :type Integer) (bFromSweep :type Boolean) (SweepResult :type "HitResult Structure (by ref)"))
  (bind _ascharacter_paper_player (cast `/Game/BP_player/character_paper_player` OtherActor))
  (add `/Game/BP_player/character_paper_player.use_player` _ascharacter_paper_player (delegate `player_press_use`))
  (`self.info_press`)
  (set `self.is_near_table` true))

(event `self.collider.OnComponentEndOverlap`
  (params (OverlappedComponent :type "PrimitiveComponent Object Reference") (OtherActor :type "Actor Object Reference") (OtherComp :type "PrimitiveComponent Object Reference") (OtherBodyIndex :type Integer))
  (bind _ascharacter_paper_player (cast `/Game/BP_player/character_paper_player` OtherActor))
  (remove `/Game/BP_player/character_paper_player.use_player` _ascharacter_paper_player (delegate `player_press_use`))
  (set `self.is_near_table` false)
  (`Widget.SetVisibility` (`self.w_text`) "Hidden"))

(event `player_press_use`
  (if (`self.is_near_table`)
    (`Widget.SetVisibility` (`self.w_text`) "Visible")))

(fn `info_press`
  (bind _asinfo_door_lock (cast `/Game/interaction/door_lock/info_door_lock` (`WidgetComponent.GetUserWidgetObject` (`self.widget_info`))))
  (`Widget.SetVisibility` _asinfo_door_lock "Visible")
  (`/Game/interaction/door_lock/info_door_lock.set_text` _asinfo_door_lock (`KismetStringLibrary.Concat_StrStr` "press key(" (`KismetTextLibrary.Conv_TextToString` (`KismetInputLibrary.Key_GetDisplayName` (`.Key` (break `InputActionKeyMapping` (`|GetArrayItem` (`InputSettings.GetActionMappingByName` (`InputSettings.GetInputSettings`) "use")))))) ")"))
  (`/Game/interaction/door_lock/info_door_lock.falloff_text` _asinfo_door_lock true)
  (`KismetSystemLibrary.K2_SetTimer` null "reset_info" 4.0))

(fn `reset_info`
  (bind _asinfo_door_lock (cast `/Game/interaction/door_lock/info_door_lock` (`WidgetComponent.GetUserWidgetObject` (`self.widget_info`))))
  (`/Game/interaction/door_lock/info_door_lock.falloff_text` _asinfo_door_lock false))

(fn `UserConstructionScript`)