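; Vertical ladder actor that puts the 2D paper player into and out of a ladder state.
; The construction script stacks non-colliding Paper2D sprites at a fixed offset to span the height between the top and bottom points.
; It also scales and centres a trigger box on that height.
; Box overlap begin and end call OnLadder and OffLadder on the player character.
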(event `self.Box.OnComponentBeginOverlap`
  (params (OverlappedComponent :type "PrimitiveComponent Object Reference") (OtherActor :type "Actor Object Reference") (OtherComp :type "PrimitiveComponent Object Reference") (OtherBodyIndex :type Integer) (bFromSweep :type Boolean) (SweepResult :type "HitResult Structure (by ref)"))
  (bind _ascharacter_paper_player (cast `/Game/BP_player/character_paper_player` OtherActor))
  (`/Game/BP_player/character_paper_player.on_ladder` _ascharacter_paper_player))

(event `self.Box.OnComponentEndOverlap`
  (params (OverlappedComponent :type "PrimitiveComponent Object Reference") (OtherActor :type "Actor Object Reference") (OtherComp :type "PrimitiveComponent Object Reference") (OtherBodyIndex :type Integer))
  (bind _ascharacter_paper_player (cast `/Game/BP_player/character_paper_player` OtherActor))
  (`/Game/BP_player/character_paper_player.off_ladder` _ascharacter_paper_player))

(fn `UserConstructionScript`
  (bind _ladder_offset (`self.ladder_offset`))
  (bind _box (`self.Box`))
  (bind (_returnvalue_x _returnvalue_y _returnvalue_z) (`KismetMathLibrary.BreakVector` (- (`self.ladder_top`) (`self.ladder_bottom`))))
  (for _index (range (+ (`KismetMathLibrary.FTrunc` (/ _returnvalue_z _ladder_offset)) 1))
    (bind _returnvalue (`AddComponent|NODE_AddPaperSpriteComponent-0` :`RelativeTransform` (`KismetMathLibrary.MakeTransform` (`KismetMathLibrary.MakeVector` 0.0 0.0 (* _index _ladder_offset)))))
    (`PrimitiveComponent.SetCollisionEnabled` _returnvalue "NoCollision")
    (`PaperSpriteComponent.SetSprite` _returnvalue (`self.sprite_list`)))
  (`SceneComponent.SetRelativeScale3D` _box (`KismetMathLibrary.MakeVector` 1.0 1.0 (/ _returnvalue_z (* _ladder_offset 2.0))))
  (`SceneComponent.K2_SetRelativeLocation` _box (`KismetMathLibrary.MakeVector` 0.0 0.0 (/ _returnvalue_z 2.0)) false false))