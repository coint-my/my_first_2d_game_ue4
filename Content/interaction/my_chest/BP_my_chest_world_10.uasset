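; A world chest actor that swallows dropped item actors and lets the player loot them through a chest UI, destroying itself once looted empty.
; Items overlapping its item collision, re-enabled shortly after BeginPlay, are saved as structs in a small capped array and destroyed.
; The player's use event opens the widget while in range.
; Taking an item spawns a temporary item actor to pass into the player's inventory component, removing the entry on success.
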(event `self.ReceiveBeginPlay`
  (bind _ascharacter_paper_player (cast `/Game/BP_player/character_paper_player` (`GameplayStatics.GetPlayerPawn` 0)))
  (add `/Game/BP_player/character_paper_player.use_player` _ascharacter_paper_player (delegate `use_character_player`))
  (`PrimitiveComponent.SetCollisionEnabled` (`self.collision_item`) "NoCollision")
  (`KismetSystemLibrary.Delay` 0.1)
  (`PrimitiveComponent.SetCollisionEnabled` (`self.collision_item`) "QueryOnly"))

(event `use_character_player`
  (bind _returnvalue (`GameplayStatics.GetPlayerController` 0))
  (bind _my_ui_chest (`self.my_ui_chest`))
  (if (and (`self.is_player_collision`) (not (`self.is_open_ui`)))
    (bind _returnvalue_2 (`|CreateWidget` "/Game/UI/my_inventory/UI_chest_world.UI_chest_world_C" (`GameplayStatics.GetPlayerController` 0) (`self.my_stor`)))
    (bind _output_get (set `self.my_ui_chest` _returnvalue_2))
    (`UserWidget.AddToViewport` _output_get 0)
    (set `self.is_open_ui` true)
    (`WidgetBlueprintLibrary.SetInputMode_UIOnlyEx` _returnvalue _output_get "LockAlways")
    (set `PlayerController.bShowMouseCursor` true _returnvalue)
    (add `Button.OnClicked` (`/Game/UI/my_inventory/UI_chest_world.Button_close` _my_ui_chest) (delegate `my_close_event`))
    (add `/Game/UI/my_inventory/UI_chest_world.my_take_event` _my_ui_chest (delegate `my_take_item`))))

(event `my_take_item`
  (params (my_item :type "/Game/UI/my_inventory/UI_chest_item Object Reference"))
  (bind _my_struct (`/Game/UI/my_inventory/UI_chest_item.my_struct` my_item))
  (bind _returnvalue (`|SpawnActorFromClass` "/Game/items/my_item_world/BP_my_item_world.BP_my_item_world_C" (`KismetMathLibrary.MakeTransform` (0.0 0.0 0.0)) "Undefined" "OverrideRootScale" null (`.my_source_2_33CE7E01467181A544CD8F8571A376EC` (break `/Game/UI/my_inventory/my_chest_storage` _my_struct)) null))
  (bind _count (`/Game/UI/my_inventory/UI_chest_item.my_get_count` my_item))
  (set `/Game/items/my_item_world/COM_my_inventory_count.my_count` _count (`self.GetComponentByClass` _returnvalue "/Game/items/my_item_world/COM_my_inventory_count.COM_my_inventory_count_C"))
  (bind _val (`/Game/items/my_item_world/COM_my_inventary.my_add_inventory` (`self.GetComponentByClass` (`self.my_player`) "/Game/items/my_item_world/COM_my_inventary.COM_my_inventary_C") _returnvalue))
  (`self.K2_DestroyActor` _returnvalue)
  (if _val
    (`Widget.RemoveFromParent` my_item)
    (`KismetArrayLibrary.Array_RemoveItem` (`self.my_stor`) _my_struct)
    (if (== (`KismetArrayLibrary.Array_Length` (`self.my_stor`)) 0)
      (`self.my_close_event`)
      (`self.K2_DestroyActor`))))

(event `my_close_event`
  (bind _returnvalue (`GameplayStatics.GetPlayerController` 0))
  (set `self.is_open_ui` false)
  (`Widget.RemoveFromParent` (`self.my_ui_chest`))
  (`WidgetBlueprintLibrary.SetInputMode_GameOnly` _returnvalue)
  (set `PlayerController.bShowMouseCursor` false _returnvalue))

(event `self.collision.OnComponentBeginOverlap`
  (params (OverlappedComponent :type "PrimitiveComponent Object Reference") (OtherActor :type "Actor Object Reference") (OtherComp :type "PrimitiveComponent Object Reference") (OtherBodyIndex :type Integer) (bFromSweep :type Boolean) (SweepResult :type "HitResult Structure (by ref)"))
  (bind _ascharacter_paper_player (cast `/Game/BP_player/character_paper_player` OtherActor))
  (set `self.my_player` _ascharacter_paper_player)
  (set `self.is_player_collision` true))

(event `self.collision.OnComponentEndOverlap`
  (params (OverlappedComponent :type "PrimitiveComponent Object Reference") (OtherActor :type "Actor Object Reference") (OtherComp :type "PrimitiveComponent Object Reference") (OtherBodyIndex :type Integer))
  (cast `/Game/BP_player/character_paper_player` OtherActor)
  (set `self.my_player` null)
  (set `self.is_player_collision` false))

(event `self.collision_item.OnComponentBeginOverlap`
  (params (OverlappedComponent :type "PrimitiveComponent Object Reference") (OtherActor :type "Actor Object Reference") (OtherComp :type "PrimitiveComponent Object Reference") (OtherBodyIndex :type Integer) (bFromSweep :type Boolean) (SweepResult :type "HitResult Structure (by ref)"))
  (bind _asbp_my_item_world (cast `/Game/items/my_item_world/BP_my_item_world` OtherActor))
  (bind _val (`self.my_try_create_item` _asbp_my_item_world))
  (`KismetSystemLibrary.Delay` 0.05)
  (if _val
    (`self.K2_DestroyActor` OtherActor)
    (else
      (`KismetSystemLibrary.PrintString` "is full chest"))))

(fn `my_try_create_item`
  (params (item :type "/Game/items/my_item_world/BP_my_item_world Object Reference"))
  (returns (val :type Boolean))
  (if (< (`KismetArrayLibrary.Array_Length` (`self.my_stor`)) 7)
    (`KismetArrayLibrary.Array_Add` (`self.my_stor`) (make `/Game/UI/my_inventory/my_chest_storage` (`/Game/items/my_item_world/BP_my_item_world.my_struct_object` item) (`/Game/items/my_item_world/COM_my_inventory_count.my_count` (`self.GetComponentByClass` item "/Game/items/my_item_world/COM_my_inventory_count.COM_my_inventory_count_C"))))
    (return true)
    (else
      (return false))))

(fn `UserConstructionScript`)