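; Test enemy projectile that trails smoke and explodes when it hits the player.
; On BeginPlay it attaches a smoke emitter to its Box, whose overlap with the paper player character destroys the actor.
; The explosion lives in Destroyed, so any destruction applies radial damage with a custom damage type, plus sparks and a bomb sound.
; The RadialForce component's radius sets the damage radius.
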(event `self.ReceiveBeginPlay`
  (bind _box (`self.Box`))
  (`GameplayStatics.SpawnEmitterAttached` "/Game/particle/my_test_smoke/P_my_test_smoke.P_my_test_smoke" _box "None" (`SceneComponent.K2_GetComponentLocation` _box) (struct) (0.5 0.5 0.5) "KeepWorldPosition"))

(event `self.Box.OnComponentBeginOverlap`
  (params (OverlappedComponent :type "PrimitiveComponent Object Reference") (OtherActor :type "Actor Object Reference") (OtherComp :type "PrimitiveComponent Object Reference") (OtherBodyIndex :type Integer) (bFromSweep :type Boolean) (SweepResult :type "HitResult Structure (by ref)"))
  (cast `/Game/BP_player/character_paper_player` OtherActor)
  (`self.K2_DestroyActor`))

(event `self.ReceiveDestroyed`
  (bind _returnvalue (`SceneComponent.K2_GetComponentLocation` (`self.Box`)))
  (`GameplayStatics.ApplyRadialDamage` :`BaseDamage` 10.0 :`Origin` (`self.K2_GetActorLocation`) :`DamageRadius` (`RadialForceComponent.Radius` (`self.RadialForce`)) :`DamageTypeClass` "/Game/interaction/barrel_explode/BP_my_dame_type.BP_my_dame_type_C" :`DamageCauser` self :`InstigatedByController` (`AIBlueprintHelperLibrary.GetAIController` self))
  (`GameplayStatics.SpawnEmitterAtLocation` "/Game/particle/sparks/P_my_spark_01.P_my_spark_01" _returnvalue (struct) (1.0 1.0 1.0) true "AutoRelease")
  (`GameplayStatics.PlaySoundAtLocation` "/Game/sound/explode/S_my_the_bomb.S_my_the_bomb" _returnvalue (struct) 1.0 1.0 0.0 null null null))

(fn `UserConstructionScript`)