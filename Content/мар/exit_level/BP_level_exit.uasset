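; Level exit actor that loads the tr_tittle level on any overlap with its Exit component and also hosts the in-game pause menu.
; BeginPlay stores NextLevel in the game instance and creates hidden menu and settings widgets.
; show_game_menu plays four timelines that slide buttons in from different sides; the settings timeline's finish pauses the game and binds Resume and Settings.
; Resume unpauses and reverses the slide, while Settings swaps to the settings widget until Back.
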(event `self.ReceiveBeginPlay`
  (bind _asmy_game_instance (cast `/Game/myGameMode/myGameInstance` (`GameplayStatics.GetGameInstance`)))
  (bind _output_get (set `self.g_instance` _asmy_game_instance))
  (set `/Game/myGameMode/myGameInstance.next_level` (`self.next_level`) _output_get)
  (bind _returnvalue (`|CreateWidget` "/Game/UI/game_menu.game_menu_C"))
  (bind _output_get_2 (set `self.widget_game_menu` _returnvalue))
  (`UserWidget.AddToViewport` _output_get_2 0)
  (`self.show` false)
  (bind _returnvalue_2 (`|CreateWidget` "/Game/UI/game_settings.game_settings_C"))
  (bind _output_get_3 (set `self.widget_settings` _returnvalue_2))
  (`UserWidget.AddToViewport` _output_get_3 0)
  (`self.show_settings` false))

(event `self.exit.OnComponentBeginOverlap`
  (params (OverlappedComponent :type "PrimitiveComponent Object Reference") (OtherActor :type "Actor Object Reference") (OtherComp :type "PrimitiveComponent Object Reference") (OtherBodyIndex :type Integer) (bFromSweep :type Boolean) (SweepResult :type "HitResult Structure (by ref)"))
  (`GameplayStatics.OpenLevel` "tr_tittle"))

(event `bind_buttom`
  (bind _widget_game_menu (`self.widget_game_menu`))
  (add `/Game/UI/game_menu.my_event_resume` _widget_game_menu (delegate `CustomEvent`))
  (`GameplayStatics.SetGamePaused` true)
  (set `PlayerController.bShowMouseCursor` true (`GameplayStatics.GetPlayerController` 0))
  (add `/Game/UI/game_menu.my_event_settings` _widget_game_menu (delegate `CustomEvent_0`)))

(event `show_game_menu`
  (`self.show` true)
  (`self.m_play_menu`))

(event `CustomEvent_0`
  (`Widget.SetVisibility` (`self.widget_game_menu`) "Hidden")
  (`self.show_settings` true)
  (add `/Game/UI/game_settings.event_back_button` (`self.widget_settings`) (delegate `CustomEvent_2`)))

(event `CustomEvent`
  (`GameplayStatics.SetGamePaused` false)
  (set `PlayerController.bShowMouseCursor` false (`GameplayStatics.GetPlayerController` 0))
  (`self.m_reverse_menu`)
  (`KismetSystemLibrary.Delay` 0.5)
  (`self.show` false))

(event `CustomEvent_2`
  (`self.show_settings` false)
  (`Widget.SetVisibility` (`self.widget_game_menu`) "Visible"))

(fn `setting_animation`
  (params (location :type "Vector Structure") (delta :type "Float (double-precision)") (widget_gameMenu :type "ContentWidget Object Reference"))
  (bind (_rendertransform_translation _rendertransform_scale _rendertransform_shear _rendertransform_angle) (break `WidgetTransform` (`Widget.RenderTransform` widget_gameMenu)))
  (`Widget.SetRenderTransform` widget_gameMenu (make `WidgetTransform` (`KismetMathLibrary.Conv_VectorToVector2D` (`KismetMathLibrary.VLerp` location (0.0 0.0 0.0) delta)) _rendertransform_scale _rendertransform_shear _rendertransform_angle)))

(fn `show`
  (params (isShow :type Boolean))
  (bind _returnvalue (`GameplayStatics.GetPlayerController` 0))
  (bind _widget_game_menu (`self.widget_game_menu`))
  (if isShow
    (`Widget.SetVisibility` _widget_game_menu "Visible")
    (`WidgetBlueprintLibrary.SetInputMode_UIOnlyEx` _returnvalue (`self.widget_game_menu`))
    (else
      (`Widget.SetVisibility` _widget_game_menu "Hidden")
      (`WidgetBlueprintLibrary.SetInputMode_GameOnly` _returnvalue)
      (`GameplayStatics.SetGamePaused` false)
      (set `PlayerController.bShowMouseCursor` false _returnvalue))))

(fn `show_settings`
  (params (show :type Boolean))
  (bind _widget_settings (`self.widget_settings`))
  (if show
    (`Widget.SetVisibility` _widget_settings "Visible")
    (else
      (`Widget.SetVisibility` _widget_settings "Hidden"))))

(fn `UserConstructionScript`)