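; A world item actor that merges with another item of its own class into a chest when the two overlap.
; After a short delay, the overlap event spawns a BP_my_chest_world_10 at the CollisionBox location with a fixed Y coordinate.
; It passes the other item, then itself, to the chest's MyTryCreateItem, destroying each on success and printing an error on failure.
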(event `self.collision_item.OnComponentBeginOverlap`
  (params (OverlappedComponent :type "PrimitiveComponent Object Reference") (OtherActor :type "Actor Object Reference") (OtherComp :type "PrimitiveComponent Object Reference") (OtherBodyIndex :type Integer) (bFromSweep :type Boolean) (SweepResult :type "HitResult Structure (by ref)"))
  (bind (_returnvalue_x _returnvalue_y _returnvalue_z) (`KismetMathLibrary.BreakVector` (`SceneComponent.K2_GetComponentLocation` (`self.collision_box`))))
  (bind _asbp_my_item_world (cast `/Game/items/my_item_world/BP_my_item_world` OtherActor))
  (set `self.my_temp_item_world` _asbp_my_item_world)
  (`KismetSystemLibrary.Delay` 0.1)
  (bind _returnvalue (`|SpawnActorFromClass` "/Game/interaction/my_chest/BP_my_chest_world_10.BP_my_chest_world_10_C" (`KismetMathLibrary.MakeTransform` (`KismetMathLibrary.MakeVector` _returnvalue_x -4.0 _returnvalue_z) (struct) (0.8 0.8 0.8)) "Undefined" "OverrideRootScale" null (`GameplayStatics.GetPlayerPawn` 0)))
  (bind _val (`/Game/interaction/my_chest/BP_my_chest_world_10.my_try_create_item` _returnvalue (`self.my_temp_item_world`)))
  (if _val
    (`self.K2_DestroyActor` (`self.my_temp_item_world`))
    (bind _val_2 (`/Game/interaction/my_chest/BP_my_chest_world_10.my_try_create_item` _returnvalue self))
    (if _val_2
      (`self.K2_DestroyActor`)
      (else
        (`KismetSystemLibrary.PrintString` "error bp_my_item_world" :!label _label)))
    (else
      (goto _label))))

(fn `UserConstructionScript`)