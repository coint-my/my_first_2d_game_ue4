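; BP_my_item_heal is a healing pickup that the paper player character collects by touching it.
; Its box collision overlap casts to character_paper_player and passes the item's HaveHeal value to that character's HaveHeal function.
; It then spawns an auto-released particle effect, plays a heal sound at its location and destroys itself.
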(event `self.Box collision.OnComponentBeginOverlap`
  (params (OverlappedComponent :type "PrimitiveComponent Object Reference") (OtherActor :type "Actor Object Reference") (OtherComp :type "PrimitiveComponent Object Reference") (OtherBodyIndex :type Integer) (bFromSweep :type Boolean) (SweepResult :type "HitResult Structure (by ref)"))
  (bind _returnvalue (`self.K2_GetActorLocation`))
  (bind _ascharacter_paper_player (cast `/Game/BP_player/character_paper_player` OtherActor))
  (`/Game/BP_player/character_paper_player.have_heal` _ascharacter_paper_player (`self.have_heal`))
  (`GameplayStatics.SpawnEmitterAtLocation` "/Game/particle/my_item_heal/P_item_heal.P_item_heal" _returnvalue (struct) (2.0 2.0 2.0) true "AutoRelease")
  (`GameplayStatics.PlaySoundAtLocation` "/Game/sound/items/S_heal_up.S_heal_up" _returnvalue (struct) 1.0 1.0 0.0 null null null)
  (`self.K2_DestroyActor`))

(fn `UserConstructionScript`
  (`parent.UserConstructionScript`))